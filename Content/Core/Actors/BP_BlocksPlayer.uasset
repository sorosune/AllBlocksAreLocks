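; BP_BlocksPlayer is a player Blueprint whose graph handles only the pause menu toggle.
; BeginPlay creates and stores a WB_PauseMenu widget for reuse.
; Escape drives a FlipFlop that alternately adds or removes the menu and shows or hides player controller 0's mouse cursor.
; Both branches toggle game pause through the "pause" console command rather than setting an explicit paused state.
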(event `self.ReceiveBeginPlay`
  (bind _returnvalue (`|CreateWidget` "/Game/Core/UI/WB_PauseMenu.WB_PauseMenu_C"))
  (set `self.PauseMeny` _returnvalue))

(event `Key|Escape` :paused true
  (params (Key :type "Key Structure"))
  (:`Pressed`
    (`/Engine/EditorBlueprintResources/StandardMacros.FlipFlop`
      (:`A`
        (`UserWidget.AddToViewport` (`self.PauseMeny`) 0)
        (set `PlayerController.bShowMouseCursor` true (`GameplayStatics.GetPlayerControllerFromID` 0))
        (`KismetSystemLibrary.ExecuteConsoleCommand` "pause" null))
      (:`B`
        (`Widget.RemoveFromParent` (`self.PauseMeny`))
        (set `PlayerController.bShowMouseCursor` false (`GameplayStatics.GetPlayerControllerFromID` 0))
        (`KismetSystemLibrary.ExecuteConsoleCommand` "pause" null)))))

(fn `UserConstructionScript`)